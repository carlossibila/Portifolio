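; BP_masterActorPickUp is a collectible pickup actor with a dot or power type.
; When the player character overlaps its sphere collision, it increases that character's count by type, triggers the power pickup response for power types, then destroys itself.
; The construction script switches on the same type to set the mesh scale for power pickups.
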(event `self.SphereCollision.OnComponentBeginOverlap`
  (params (OverlappedComponent :type "PrimitiveComponent Object Reference") (OtherActor :type "Actor Object Reference") (OtherComp :type "PrimitiveComponent Object Reference") (OtherBodyIndex :type Integer) (bFromSweep :type Boolean) (SweepResult :type "HitResult Structure (by ref)"))
  (bind _pickuptype (`self.pickUpType`))
  ;[1 1 1] pickup destroy actor
  (bind _asbp_third_person_character_player (cast `/Game/ThirdPerson/Blueprints/BP_ThirdPersonCharacter_Player` OtherActor))
  (bind _output_get (set `self.As BP Third Person Character Player` _asbp_third_person_character_player))
  (`/Game/ThirdPerson/Blueprints/BP_ThirdPersonCharacter_Player.increaseCount` _output_get _pickuptype)
  (switch `/Game/to_portifolio/E_pickUpType` _pickuptype
    (:`NewEnumerator0`
      _)
    (:`NewEnumerator1`
      (`/Game/ThirdPerson/Blueprints/BP_ThirdPersonCharacter_Player.collectedPowerPickUp` (`self.As BP Third Person Character Player`))))
  (`/Engine/EditorBlueprintResources/StandardMacros.IsValid` self
    (:`Is Valid`
      (`self.K2_DestroyActor`))))

(fn `UserConstructionScript`
  (switch `/Game/to_portifolio/E_pickUpType` (`self.pickUpType`)
    (:`NewEnumerator0`
      _)
    (:`NewEnumerator1`
      (`SceneComponent.SetWorldScale3D` (`self.StaticMesh`) (0.5 0.5 0.5))))
  (`parent.UserConstructionScript`))