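; Base geometry actor that configures itself as a floor or wall piece from its GeometryType value.
; The construction script assigns a plane mesh for floors or a cube mesh raised along Z for walls, and sets a per-type Color variable.
; It calls the parent construction script afterwards; Color is not applied to a material here, and the event graph holds only disabled default events.
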(fn `UserConstructionScript`
  (bind _staticmesh (`self.StaticMesh`))
  (switch `/Game/to_portifolio/E_geometryType` (`self.geometryType`)
    (:`NewEnumerator0`
      (`StaticMeshComponent.SetStaticMesh` (`self.StaticMesh`) "/Engine/BasicShapes/Plane.Plane")
      (set `self.color` (struct :`R` 0.078125 :`G` 0.078125 :`B` 0.078125 :`A` 1.0)))
    (:`NewEnumerator1`
      (`StaticMeshComponent.SetStaticMesh` _staticmesh "/Engine/BasicShapes/Cube1.Cube1")
      (`SceneComponent.K2_AddWorldOffset` _staticmesh (0.0 0.0 50.0) false false)
      (set `self.color` (struct :`G` 0.058628 :`B` 0.328125 :`A` 1.0))))
  (`parent.UserConstructionScript`))